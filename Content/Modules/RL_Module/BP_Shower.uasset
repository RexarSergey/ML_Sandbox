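; BP_Shower is a shower actor that starts at a random temperature and shows it through the roll of its Cube component.
; BeginPlay sets a length, picks an integer temperature, stores the cube's starting roll, then calls UpdateRotation.
; UpdateRotation linearly maps a 0–100 temperature onto a half-turn of roll centred on zero, preserving pitch and yaw.
; The stored starting roll does not affect the applied rotation.
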(event EventBeginPlay
  (Variables|Default|Setlength 60)
  (Variables|Default|SetTemperature (Math|Random|RandomIntegerinRange 36 52))
  (Variables|Default|SetStartRot (.roll (Variables|/Script/Engine.SceneComponent|GetRelativeRotation (Variables|Default|GetCube))))
  (CallFunction|UpdateRotation))

(event Collision|EventActorBeginOverlap
  (params (OtherActor :type Actor%20Object%20Reference)))

(event EventTick
  (params (DeltaSeconds :type Float%20%28single-precision%29)))

(fn ConstructionScript)

(fn UpdateRotation
  (bind _cube (Variables|Default|GetCube))
  (bind _relativerotation (Variables|/Script/Engine.SceneComponent|GetRelativeRotation _cube))
  (LocalVariables|SetX (.roll _relativerotation))
  (Transformation|SetRelativeRotation _cube (Math|Rotator|MakeRotator (- (* (/ (Math|Conversions|ToFloat(Integer) (Variables|Default|GetTemperature)) 1e+02) 1.8e+02) 9e+01) (.pitch _relativerotation) (.yaw _relativerotation)) false false))