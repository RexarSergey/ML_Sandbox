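; BP_Goal is an arena goal trigger for tournament matches that reports the first player to reach it.
; It arms two seconds after BeginPlay, then a box overlap passes the actor to the Server event.
; That event resolves the character's tournament controller, sends it to the game mode's UpdateMatchResult and disarms the goal.
; Older ServerWon and PlayerWon calls remain unconnected.
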(event OnComponentBeginOverlap(Box)
  (params (OverlappedComponent :type Primitive%20Component%20Object%20Reference) (OtherActor :type Actor%20Object%20Reference) (OtherComp :type Primitive%20Component%20Object%20Reference) (OtherBodyIndex :type Integer) (bFromSweep :type Boolean) (SweepResult :type Hit%20Result%20Structure%20%28by%20ref%29))
  (if (Variables|Default|GetIsAvable)
    (CallFunction|Server OtherActor)))

(event Custom|Server
  (params (Other%20Actor :type Actor%20Object%20Reference))
  (bind _asbp_third_person_character (Utilities|Casting|CastToBP_ThirdPersonCharacter Other%20Actor))
  (bind _asbp_tournament_player_controller (Utilities|Casting|CastToBP_Tournament_PlayerController (Pawn|GetController _asbp_third_person_character)))
  (bind _asbp_tournament_game_mode (Utilities|Casting|CastToBP_Tournament_GameMode (Game|GetGameMode)))
  (Default|UpdateMatchResult _asbp_tournament_game_mode _asbp_tournament_player_controller)
  (Variables|Default|SetIsAvable false))

(event EventBeginPlay
  (Utilities|FlowControl|Delay 2.0)
  (Variables|Default|SetIsAvable true))

(fn ConstructionScript)