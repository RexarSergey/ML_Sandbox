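; HUD Blueprint for the SoloTask map that controls the display of its start menu.
; BeginPlay caches the StartMenu widget from ACStartMenuW.
; DrawStartMenu adds it to the viewport and sets Game and UI input focused on it.
; DeleteStartMenu switches the menu's widget switcher to its second page and restores game-only input, leaving the widget in the viewport because the RemoveFromParent node is disconnected.
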(event Custom|Delete%20StartMenu
  (Utilities|IsValid (Variables|Default|GetStart%20Menu)
    (:Is%20Valid
      (Class|WidgetSwitcher|SetActiveWidgetIndex (Variables|/Game/Modules/AM_Module/Maps/SoloTask/UI/WBP_StartMenu.WBP_StartMenu_C|GetWidgetSwitcher_166 (Variables|Default|GetStart%20Menu)) 1)
      (Utilities|IsValid (Game|Player|GetOwningPlayerController)
        (:Is%20Valid
          (Input|SetInputModeGameOnly (Game|Player|GetOwningPlayerController) false))))))

(event Custom|Draw%20StartMenu
  (bind _start_menu (Variables|Default|GetStart%20Menu))
  (Utilities|IsValid _start_menu
    (:Is%20Valid
      (UserInterface|Viewport|AddtoViewport _start_menu 0)
      (Utilities|IsValid (Game|Player|GetOwningPlayerController)
        (:Is%20Valid
          (Input|SetInputModeGameandUI (Game|Player|GetOwningPlayerController) (Variables|Default|GetStart%20Menu) "DoNotLock" false false))))))

(event EventBeginPlay
  (Variables|Default|SetStart%20Menu (Variables|/Game/Modules/AM_Module/Maps/SoloTask/UI/AC_StartMenuW.AC_StartMenuW_C|GetStartMenu (Variables|Default|GetAC_StartMenuW))))

(fn ConstructionScript)