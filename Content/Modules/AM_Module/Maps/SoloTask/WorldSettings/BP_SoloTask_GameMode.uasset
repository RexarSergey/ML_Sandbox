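; Game mode for the SoloTask map that runs a ready-up lobby and starts the match.
; On BeginPlay, unless the save game flags a listen server, it creates local players up to the saved maximum.
; Logins and ready changes update parallel player and ready arrays, then refresh every controller's lobby display.
; ServerStartMatch closes start menus, spawns characters on the arena and syncs their transforms to controllers; AllPlayersReady aggregates ready flags.
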(event Custom|Set%20Player%20Is%20Ready
  (params (Player%20Controller :type Player%20Controller%20Object%20Reference) (Is%20Ready :type Boolean))
  (Utilities|Array|SetArrayElem (Variables|Default|GetIsReady) (Utilities|Array|FindItem (Variables|Default|GetPlayersList) Player%20Controller) Is%20Ready)
  (CallFunction|UpdateLobby))

(event Custom|Update%20Lobby
  (for _array_element (Variables|Default|GetPlayersList)
    (bind _asbp_solo_task_player_controller (Utilities|Casting|CastToBP_SoloTask_PlayerController _array_element))
    (Default|UpdatePlayerReady _asbp_solo_task_player_controller)))

(event Custom|Server%20Start%20Match
  (for _array_element (Variables|Default|GetPlayersList)
    (bind _asbp_solo_task_player_controller (Utilities|Casting|CastToBP_SoloTask_PlayerController _array_element))
    (Default|CloseStartMenu _asbp_solo_task_player_controller)
    (bind _asbp_third_person_character (Utilities|Casting|CastToBP_ThirdPersonCharacter (Pawn|GetControlledPawn _asbp_solo_task_player_controller)))
    (Class|PDPTasksCharacter|SpawnonArena _asbp_third_person_character)
    (Default|UpdateLoc/Rot _asbp_solo_task_player_controller (Transformation|GetActorLocation (Pawn|GetControlledPawn _asbp_solo_task_player_controller)) (Transformation|GetActorRotation (Pawn|GetControlledPawn _asbp_solo_task_player_controller)))))

(event EventBeginPlay
  (Utilities|FlowControl|Delay 0.2)
  (bind _asbp_game_instance (Utilities|Casting|CastToBP_GameInstance (Game|GetGameInstance)))
  (if (not (Variables|/Game/Modules/AM_Module/Frameworks/BP_SaveGame.BP_SaveGame_C|GetIsListenServer (Variables|/Game/Modules/AM_Module/Frameworks/BP_GameInstance.BP_GameInstance_C|GetSaveGame _asbp_game_instance)))
    (for _index (range 0 (- (Variables|/Game/Modules/AM_Module/Frameworks/BP_SaveGame.BP_SaveGame_C|GetMaxPlayers (Variables|/Game/Modules/AM_Module/Frameworks/BP_GameInstance.BP_GameInstance_C|GetSaveGame _asbp_game_instance)) 1))
      (Class|GameplayStatics|CreatePlayer _index))))

(event EventPostLogin
  (params (NewPlayer :type Player%20Controller%20Object%20Reference))
  (Utilities|Array|Add (Variables|Default|GetPlayersList) NewPlayer)
  (Utilities|Array|Add (Variables|Default|GetIsReady) false)
  (CallFunction|UpdateLobby))

(fn ConstructionScript)

(fn AllPlayersReady
  (for _array_element (Variables|Default|GetIsReady)
    (LocalVariables|SetResult (and _array_element (LocalVariables|GetResult))))
  (return (LocalVariables|GetResult)))