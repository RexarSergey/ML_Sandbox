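; Lobby game mode that tracks connected players, their profiles and ready states, and pushes lobby updates to them.
; On the Lobby level, a new player is sent away if the GameInstance's max player count is reached, otherwise registered and given the lobby menu.
; Players and ready flags live in index-matched arrays, pruned on logout.
; UpdateLobby selectively sends names, selected level and readiness to every player controller.
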(event Custom|Update%20Lobby
  (params (Player%20Names :type Boolean) (LevelSelection :type Boolean) (PlayersReady :type Boolean))
  (if Player%20Names
    ;[1 1 1] Refresh Player Profoles in Server
    (Utilities|Array|Clear (Variables|Default|GetAllPlayerProfiles))
    (for _array_element (Variables|Default|GetAllConnectedPlayers)
      (Utilities|Array|Add (Variables|Default|GetAllPlayerProfiles) (Variables|/Game/Modules/AM_Module/Maps/Lobby/WorldSettings/BP_Lobby_PlayerController.BP_Lobby_PlayerController_C|GetPlayer%20Profile _array_element))))
  (for _array_element_2 (Variables|Default|GetAllConnectedPlayers)
    (if Player%20Names
      (Default|UpdatePlayerNames _array_element_2 (Variables|Default|GetAllPlayerProfiles)))
    (if LevelSelection
      (Default|UpdateLevelSelection _array_element_2 (Variables|Default|GetSelectedLevelName)))
    (if PlayersReady
      (Default|UpdatePlayerReady _array_element_2 (Variables|Default|GetIsPlayerReady)))))

(event Custom|Set%20Player%20Ready
  (params (PlayerController :type BP%20Lobby%20Player%20Controller%20Object%20Reference) (IsReady :type Boolean))
  (Utilities|Array|SetArrayElem (Variables|Default|GetIsPlayerReady) (Utilities|Array|FindItem (Variables|Default|GetAllConnectedPlayers) PlayerController) IsReady)
  (CallFunction|UpdateLobby false false true))

(event EventOnLogout
  (params (ExitingController :type Controller%20Object%20Reference))
  (bind _asbp_lobby_player_controller (Utilities|Casting|CastToBP_Lobby_PlayerController ExitingController))
  ;[1 1 1] Remove user from list
  (Utilities|Array|RemoveIndex (Variables|Default|GetIsPlayerReady) (Utilities|Array|FindItem (Variables|Default|GetAllConnectedPlayers) _asbp_lobby_player_controller))
  (Utilities|Array|RemoveIndex (Variables|Default|GetAllConnectedPlayers) (Utilities|Array|FindItem (Variables|Default|GetAllConnectedPlayers) _asbp_lobby_player_controller))
  (CallFunction|UpdateLobby true false true))

(event EventHandleStartingNewPlayer
  (params (NewPlayer :type Player%20Controller%20Object%20Reference))
  (bind _returnvalue (Game|GetCurrentLevelName true))
  (switch string _returnvalue
    (:Lobby
      (bind _asbp_lobby_player_controller (Utilities|Casting|CastToBP_Lobby_PlayerController NewPlayer))
      (bind _bresult (CallFunction|CheckSession))
      (if _bresult
        (Default|EndClientSession _asbp_lobby_player_controller)
        (else
          ;[1 1 1] Adding new user to the list
          (bind _returnvalue_2 (Utilities|Array|Add (Variables|Default|GetAllConnectedPlayers) _asbp_lobby_player_controller))
          (Utilities|Array|SetArrayElem (Variables|Default|GetIsPlayerReady) _returnvalue_2 false true)
          ;[1 1 1] Show UI in Clients
          (Default|CreateLobbyMenu _asbp_lobby_player_controller)
          (Default|InitialSetup _asbp_lobby_player_controller))))))

(fn ConstructionScript)

(fn CheckSession
  (bind _asbp_game_instance (Utilities|Casting|CastToBP_GameInstance (Game|GetGameInstance)))
  (if (== (Variables|/Game/Modules/AM_Module/Frameworks/BP_GameInstance.BP_GameInstance_C|GetMaxPlayerNumber _asbp_game_instance) (Utilities|Array|Length (Variables|Default|GetAllConnectedPlayers)))
    (return true)
    (else
      (return false))))