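; Player controller for the multiplayer lobby, running the lobby menu and load screen UI with a UI-only cursor input mode.
; It loads or creates the saved player profile, then sends it and ready changes to BP_Lobby_GameMode through Server-prefixed events.
; Update events pass player names, level selection and ready states into the lobby menu widget.
; Ending the client session destroys it and opens MainMenu.
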(event Custom|Create%20Load%20Screen
  ;[1 1 1] Open Level and UI in Client
  (CallFunction|UIShowLoadScreen))

(event Custom|End%20Client%20Session
  ;[1 1 1] Open Level and UI in Client
  (|DestroySession (Game|GetPlayerController 0)
    (:then
      (Game|OpenLevel(byName) "MainMenu"))))

(event Custom|Create%20Lobby%20Menu
  ;[1 1 1] Open Level and UI in Client
  (CallFunction|UIShowLobbyMenu))

(event Custom|Initial%20Setup
  ;[1 1 1] Load PlayerProfile and Update new information in other Clients
  (CallFunction|LoadSavedProfile)
  (CallFunction|ServerUpdateLobby (Variables|Default|GetPlayer%20Profile)))

(event Custom|Update%20Player%20Names
  (params (PlayerProfiles :type Array%20of%20S%20Player%20Profile%20Structures))
  (bind _lobbymenu_w (Variables|Default|GetLobbyMenu_W))
  ;[1 1 1] Load PlayerProfile and Update new information in other Clients
  (Utilities|IsValid _lobbymenu_w
    (:Is%20Valid
      (Default|ClearPlayerNames _lobbymenu_w)
      (Default|UpdatePlayerNames _lobbymenu_w PlayerProfiles))))

(event Custom|Server%20Update%20Lobby
  (params (PlayerProfile :type S%20Player%20Profile%20Structure))
  ;[1 1 1] Load PlayerProfile and Update new information in other Clients
  (Variables|Default|SetPlayer%20Profile PlayerProfile)
  (bind _asbp_lobby_game_mode (Utilities|Casting|CastToBP_Lobby_GameMode (Game|GetGameMode)))
  (Default|UpdateLobby _asbp_lobby_game_mode true true true))

(event Custom|Update%20Level%20Selection
  (params (LevelRowName :type Name))
  (bind _lobbymenu_w (Variables|Default|GetLobbyMenu_W))
  ;[1 1 1] Update Host Level Selection in Clients
  (Utilities|IsValid _lobbymenu_w
    (:Is%20Valid
      (Default|UpdateLevelSelection _lobbymenu_w LevelRowName))))

(event Custom|Server%20Update%20Player%20Ready
  (params (IsReady :type Boolean))
  ;[1 1 1] Change Player Status and Update it in other Clinets
  (bind _asbp_lobby_game_mode (Utilities|Casting|CastToBP_Lobby_GameMode (Game|GetGameMode)))
  (Default|SetPlayerReady _asbp_lobby_game_mode self IsReady))

(event Custom|Update%20Player%20Ready
  (params (IsPlayersReady :type Array%20of%20Booleans))
  (bind _lobbymenu_w (Variables|Default|GetLobbyMenu_W))
  ;[1 1 1] Change Player Status and Update it in other Clinets
  (Utilities|IsValid _lobbymenu_w
    (:Is%20Valid
      (Default|UpdatePlayersReady _lobbymenu_w IsPlayersReady))))

(event EventBeginPlay
  (if (Pawn|IsLocalController)
    (Variables|Default|SetbShowMouseCursor true)
    (Input|SetInputModeUIOnly self 0 "DoNotLock" false)))

(fn ConstructionScript)

(fn UIShowLobbyMenu
  (Utilities|IsValid (Variables|Default|GetLobbyMenu_W)
    (:Is%20Valid
      _)
    (:Is%20Not%20Valid
      (bind _returnvalue (UserInterface|CreateWidget "/Game/Modules/AM_Module/Maps/Lobby/UI/WBP_LobbyMenu.WBP_LobbyMenu_C" self))
      (Variables|Default|SetLobbyMenu_W _returnvalue)))
  (UserInterface|Viewport|AddtoViewport (Variables|Default|GetLobbyMenu_W) 0)
  (return))

(fn LoadSavedProfile
  (bind _returnvalue (SaveGame|DoesSaveGameExist (LocalVariables|GetLocalSlotName)))
  (if _returnvalue
    _
    (else
      (bind _returnvalue_2 (SaveGame|CreateSaveGameObject "/Game/Modules/AM_Module/Frameworks/SG_PlayerProfile.SG_PlayerProfile_C"))
      (SaveGame|SaveGametoSlot _returnvalue_2 (LocalVariables|GetLocalSlotName))))
  (bind _returnvalue_3 (SaveGame|LoadGamefromSlot (LocalVariables|GetLocalSlotName)))
  (bind _assg_player_profile (Utilities|Casting|CastToSG_PlayerProfile _returnvalue_3))
  (Variables|Default|SetPlayer%20Profile (Variables|/Game/Modules/AM_Module/Frameworks/SG_PlayerProfile.SG_PlayerProfile_C|GetPlayerProfile _assg_player_profile))
  (return))

(fn UIShowLoadScreen
  (Viewport|RemoveAllWidgets)
  (Utilities|IsValid (Variables|Default|GetLoadScreen_W)
    (:Is%20Valid
      _)
    (:Is%20Not%20Valid
      (bind _returnvalue (UserInterface|CreateWidget "/Game/Modules/AM_Module/Maps/TravelMap/UI/WBP_LoadScreen.WBP_LoadScreen_C" self))
      (Variables|Default|SetLoadScreen_W _returnvalue)))
  (UserInterface|Viewport|AddtoViewport (Variables|Default|GetLoadScreen_W) 0)
  (return))