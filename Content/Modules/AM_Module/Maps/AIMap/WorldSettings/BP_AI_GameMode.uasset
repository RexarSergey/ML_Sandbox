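; BP_AI_GameMode is the game mode for the AI map, moving connected players to arena spawn points when matches start.
; On PostLogin it records each new player and refreshes the list of BP_ArenaComponent_SpawnPoint actors in the level.
; StartMatches teleports each player's controlled pawn to the spawn point at the same array index, copying its location and rotation, with no bounds check.
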(event Custom|Start%20Matches
  (for (_array_element _array_index) (Variables|Default|GetAllConnectedPlayers)
    (Transformation|SetActorLocationAndRotation (Pawn|GetControlledPawn _array_element) (Transformation|GetActorLocation (Utilities|Array|Get(acopy) (Variables|Default|GetSpawnPointsList) _array_index)) (Transformation|GetActorRotation (Utilities|Array|Get(acopy) (Variables|Default|GetSpawnPointsList) _array_index)))))

(event EventPostLogin
  (params (NewPlayer :type Player%20Controller%20Object%20Reference))
  (Utilities|Array|Add (Variables|Default|GetAllConnectedPlayers) NewPlayer)
  (bind _outactors (Actor|GetAllActorsOfClass "/Game/Modules/AM_Module/Blueprints/Arenas/BP_ArenaComponent_SpawnPoint.BP_ArenaComponent_SpawnPoint_C"))
  (Variables|Default|SetSpawnPointsList _outactors))

(fn ConstructionScript)